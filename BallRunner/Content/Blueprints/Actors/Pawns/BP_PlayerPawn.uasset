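; Player pawn for a rolling-ball game, steered by applying torque to the BALL component.
; Move axis inputs feed TorqueX and TorqueY, which add scaled acceleration-based torque on the perpendicular axis.
; ChangeCameraView sets spring arm length and world pitch, with no caller in this Blueprint.
; The camera fades in on BeginPlay, and any damage fades it out and reloads the current level after a short delay.
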(event `InputAxis|Move Left/Right`
  (params (AxisValue :type "Float (single-precision)"))
  (`self.TorqueY` AxisValue))

(event `InputAxis|Move Forward/Back`
  (params (AxisValue :type "Float (single-precision)"))
  (`self.TorqueX` AxisValue))

(event `self.ReceiveAnyDamage`
  (params (Damage :type "Float (single-precision)") (DamageType :type "DamageType Object Reference") (InstigatedBy :type "Controller Object Reference") (DamageCauser :type "Actor Object Reference"))
  (`self.RestartLevel`))

(event `self.ReceiveBeginPlay`
  (`PlayerCameraManager.StartCameraFade` :`self` (`GameplayStatics.GetPlayerCameraManager` 0) :`FromAlpha` 1.0 :`Duration` 2.0))

(fn `Change Camera View`
  (params (PitchSpringArm :type "Float (double-precision)") (LengthSpringArm :type "Float (double-precision)"))
  (bind _springarm (`self.SpringArm`))
  (set `SpringArmComponent.TargetArmLength` LengthSpringArm _springarm)
  (`SceneComponent.K2_SetWorldRotation` _springarm (`KismetMathLibrary.MakeRotator` 0.0 PitchSpringArm) false false))

(fn `TorqueX`
  (params (A :type "Float (double-precision)"))
  (`PrimitiveComponent.AddTorqueInRadians` (`self.BALL`) (`KismetMathLibrary.MakeVector` 0.0 (* A (`self.Multiply`))) "None" true))

(fn `TorqueY`
  (params (A :type "Float (double-precision)"))
  (`PrimitiveComponent.AddTorqueInRadians` (`self.BALL`) (`KismetMathLibrary.MakeVector` (* A (`self.Multiply`))) "None" true))

(fn `UserConstructionScript`)