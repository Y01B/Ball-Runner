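; BP_Canon is a cannon actor that fires projectiles automatically and repeatedly from BeginPlay.
; Each cycle waits for the RatFire delay, then spawns a BP_Projectile at the SpawnPoint transform, scaled by ProjectileScale.
; BarrelFireTimeline then animates the barrel's relative Y location, and its Cannon Fired event track loops execution back to the delay.
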(event `self.ReceiveBeginPlay`
  (`KismetSystemLibrary.Delay` (`self.RatFire`) :!label _label)
  (`self.SpawnProjectile`)
  (bind (_direction _barrellocationy) (`Timeline|BarrelFireTimeline` :!via `PlayFromStart`)
    (:`Update`
      (`self.CannonBarrelYLocation` _barrellocationy))
    (:`CannonFired`
      (goto _label))))

(fn `CannonBarrelYLocation`
  (params (NewLocation_Y :type "Float (double-precision)"))
  (`SceneComponent.K2_SetRelativeLocation` (`self.CannonBarrel`) (`KismetMathLibrary.MakeVector` 0.0 NewLocation_Y) false false))

(fn `SpawnProjectile`
  (`|SpawnActorFromClass` "/Game/Blueprints/Actors/Projectiles/BP_Projectile.BP_Projectile_C" (`KismetMathLibrary.MakeTransform` (`SceneComponent.K2_GetComponentLocation` (`self.SpawnPoint`)) (`SceneComponent.K2_GetComponentRotation` (`self.SpawnPoint`)) (`KismetMathLibrary.Conv_DoubleToVector` (`self.ProjectileScale`))) "AlwaysSpawn" "OverrideRootScale" null null))

(fn `UserConstructionScript`)