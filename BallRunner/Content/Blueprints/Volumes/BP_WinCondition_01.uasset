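; Level exit volume that completes the level when the player overlaps it and no BP_Crystal actors remain in the world.
; If crystals are left, it prints a Polish message saying that not all have been found.
; Completion looks up the current level name in the LevelNames array and opens the next entry, or quits the game on the last one.
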(event `self.ReceiveActorBeginOverlap`
  (params (OtherActor :type "Actor Object Reference"))
  (`/Game/Libraries/ML_Actors.IsPlayer` OtherActor
    (:`True`
      (if (`self.CheckAnyCrystals`)
        (`self.CompleteLevel`)
        (else
          (`KismetSystemLibrary.PrintString` "Nie znalazles wszystkich krysztalow"))))))

(fn `CheckAnyCrystals`
  (returns (ReturnValue :type Boolean))
  (bind _outactors (`GameplayStatics.GetAllActorsOfClass` "/Game/Blueprints/Actors/Collectibles/BP_Crystal.BP_Crystal_C"))
  (return (>= 0 (`KismetArrayLibrary.Array_Length` _outactors))))

(fn `CompleteLevel`
  (if (`self.IsFinalLvl`)
    (`KismetSystemLibrary.QuitGame` null "Quit")
    (else
      (`self.NextLevel`))))

(fn `GetCurrentIndex`
  (returns (ReturnValue :type Integer))
  (bind _returnvalue (`GameplayStatics.GetCurrentLevelName` true))
  (return (`KismetArrayLibrary.Array_Find` (`self.LevelNames`) (`KismetStringLibrary.Conv_StringToName` _returnvalue))))

(fn `IsFinalLvl`
  (returns (ReturnValue :type Boolean))
  (return (== (`KismetArrayLibrary.Array_LastIndex` (`self.LevelNames`)) (`self.GetCurrentIndex`))))

(fn `NextLevel`
  (`GameplayStatics.OpenLevel` (`|GetArrayItem` (`self.LevelNames`) (+ (`self.GetCurrentIndex`) 1))))

(fn `UserConstructionScript`)